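; Field actor that visualizes a 2D grid of blocks as debug boxes, sized by FieldSize.
; The Construction Script starts a looping one-second timer on DrawField, which loops over both axes and calls DrawBox per cell.
; Each box lasts one second and is centered via CountBlockPosition, whose graph holds only unconnected math for offsetting the root location by BlocksOffset.
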(event EventBeginPlay)

(event Collision|EventActorBeginOverlap
  (params (OtherActor :type Actor%20Object%20Reference)))

(event EventTick
  (params (DeltaSeconds :type Float%20%28single-precision%29)))

(fn ConstructionScript
  (Utilities|Time|SetTimerbyFunctionName 0 "DrawField" 1.0 true))

(fn DrawField
  (bind _fieldsize (Variables|Default|GetFieldSize))
  (for _index (range 0 (.x _fieldsize))
    (for _index_2 (range 0 (.y _fieldsize))
      (CallFunction|DrawBox _index _index_2))))

(fn DrawBox
  (params (X :type Integer) (Y :type Integer))
  (Rendering|Debug|DrawDebugBox :Center (Utilities|CountBlockPosition X Y) :Extent "30.000000,30.000000,30.000000" :Duration 1.0 :Thickness 1.0))