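; ActorsPool is an object pool that hands out actors of a Sample class for reuse.
; GetObject draws from the FreeObjects array, or spawns a new actor when the array is empty.
; Each spawned actor gets a PoolableActor component pointing back to this pool.
; ReturnObject only adds the actor back to FreeObjects, with no reset or deactivation here.
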(fn ConstructionScript)

(fn GetObject
  (bind _freeobjects (Variables|Default|GetFreeObjects))
  (bind _output (Utilities|Array|Get(acopy) _freeobjects))
  (if (> (Utilities|Array|Length (Variables|Default|GetFreeObjects)) 0)
    (Utilities|Array|RemoveItem _freeobjects _output)
    (return _output)
    (else
      (bind _returnvalue (Game|SpawnActorfromClass (Variables|Default|GetSample) (Math|Transform|MakeTransform "0, 0, 0" "0, 0, 0" "1,1,1") "Undefined" 0 0))
      (bind _returnvalue_2 (AddComponent|AddPoolableActor _returnvalue))
      (Variables|/Game/Blueprints/Components/PoolableActor.PoolableActor_C|SetPool _returnvalue_2 self)
      (return _returnvalue))))

(fn ReturnObject
  (params (ObjectToReturn :type Actor%20Object%20Reference))
  (Utilities|Array|Add (Variables|Default|GetFreeObjects) ObjectToReturn))