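; Field actor that lays out a grid of pooled blocks sized by FieldSize.
; On BeginPlay it spawns a BlocksPool, then takes an object for each cell, teleports it to CountBlockPosition and makes it visible through its HiddenActor component.
; The construction script starts a looping timer that redraws debug boxes at the same cell positions to preview the layout.
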(event EventBeginPlay
  (bind _fieldsize (Variables|Default|GetFieldSize))
  (bind _returnvalue (Game|SpawnActorfromClass "/Game/Blueprints/Actors/ActorsPool.ActorsPool_C" (Math|Transform|MakeTransform "0, 0, 0" "0, 0, 0" "1,1,1") "Undefined" 0 0))
  (bind _output_get (Variables|Default|SetBlocksPool _returnvalue))
  (for _index (range 0 (.x _fieldsize))
    (for _index_2 (range 0 (.y _fieldsize))
      (bind _object (Default|GetObject _output_get))
      (Transformation|Teleport _object (Utilities|CountBlockPosition _index _index_2) "0, 0, 0")
      (Default|SetEnabled (Actor|GetComponentbyClass _object "/Game/Blueprints/Components/HiddenActor.HiddenActor_C") true _object))))

(fn ConstructionScript
  (Utilities|Time|SetTimerbyFunctionName 0 "DebugDrawField" 1.0 true))

(fn DebugDrawField
  (bind _fieldsize (Variables|Default|GetFieldSize))
  (for _index (range 0 (.x _fieldsize))
    (for _index_2 (range 0 (.y _fieldsize))
      (CallFunction|DebugDrawBox _index _index_2))))

(fn DebugDrawBox
  (params (X :type Integer) (Y :type Integer))
  (Rendering|Debug|DrawDebugBox :Center (Utilities|CountBlockPosition X Y) :Extent "50.000000,50.000000,50.000000" :Duration 1.0 :Thickness 1.0))