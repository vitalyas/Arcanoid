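; Player-controlled plate actor that slides left and right along the Y axis, with an optional speed boost, while the game is running.
; BeginPlay saves the start position and binds handlers to the EventManager's move, boost, game-start and failure events.
; The handlers set speed and boost multiplier, which Tick applies as a swept per-frame offset without delta-time scaling.
; Failure teleports the plate back to its start and stops movement until the next start.
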(event EventBeginPlay
  (Variables|Default|SetStartPosition (Transformation|GetActorLocation))
  (bind _outactors (Actor|GetAllActorsOfClass "/Game/Blueprints/Actors/EventManager.EventManager_C"))
  (Utilities|FlowControl|Sequence
    (:then_0
      (|MoveLeftPressed (Utilities|Array|Get(acopy) _outactors)))
    (:then_1
      (|MoveLeftReleased (Utilities|Array|Get(acopy) _outactors)))
    (:then_2
      (|MoveRightPressed (Utilities|Array|Get(acopy) _outactors)))
    (:then_3
      (|MoveRightReleased (Utilities|Array|Get(acopy) _outactors)))
    (:then_4
      (|OnGameStarted (Utilities|Array|Get(acopy) _outactors)))
    (:then_5
      (|Failed (Utilities|Array|Get(acopy) _outactors)))
    (:then_6
      (|SpeedBoostPressed (Utilities|Array|Get(acopy) _outactors)))
    (:then_7
      (|SpeedBoostReleased (Utilities|Array|Get(acopy) _outactors)))))

(event EventTick
  (params (DeltaSeconds :type Float%20%28single-precision%29))
  (if (Variables|Default|GetGameStarted)
    (Transformation|AddActorWorldOffset (Math|Vector|MakeVector 0.0 (* (Variables|Default|GetCurrentSpeed) (Variables|Default|GetCurrentSpeedBoostMultiplier)) 0.0) true)))

(fn ConstructionScript)

(event Custom|OnSpeedBoostPressed
  (Variables|Default|SetCurrentSpeedBoostMultiplier (Variables|Default|GetSpeedBoostMultiplier)))

(event Custom|OnMoveLeftPressed
  (Variables|Default|SetCurrentSpeed (* (Variables|Default|GetMoveSpeed) -1.0)))

(event Custom|OnMoveLeftReleased
  (Variables|Default|SetCurrentSpeed 0.0))

(event Custom|OnMoveRightPressed
  (Variables|Default|SetCurrentSpeed (Variables|Default|GetMoveSpeed)))

(event Custom|OnMoveRightReleased
  (Variables|Default|SetCurrentSpeed 0.0))

(event Custom|OnStartGamePressed
  (Variables|Default|SetGameStarted true))

(event Custom|OnFailed
  (Transformation|Teleport (Variables|Default|GetStartPosition) "0, 0, 0")
  (Variables|Default|SetGameStarted false))

(event Custom|OnSpeedBoostReleased
  (Variables|Default|SetCurrentSpeedBoostMultiplier 1.0))