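; Object pool for Block actors that reuses returned blocks when one is requested at a position.
; ReturnObject adds an actor to FreeObjects without hiding or deactivating it.
; GetObject spawns a Block when the list is empty; otherwise it removes the first entry, then teleports whatever sits at index 0 with zero rotation.
; Because index 0 is read again after removal, the teleport targets the following entry, or none if the list empties.
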(event Custom|GetObject
  (params (Position :type Vector))
  (bind _freeobjects (Variables|Default|GetFreeObjects))
  (bind _output (Utilities|Array|Get(acopy) _freeobjects))
  (if (> (Utilities|Array|Length (Variables|Default|GetFreeObjects)) 0)
    (Utilities|Array|RemoveItem _freeobjects _output)
    (Transformation|Teleport _output Position "0, 0, 0")
    (else
      (Game|SpawnActorfromClass "/Game/Blueprints/Block.Block_C" (Math|Transform|MakeTransform Position "0, 0, 0" "1,1,1") "Undefined" 0 0))))

(event Custom|ReturnObject
  (params (Object :type Actor%20Object%20Reference))
  (Utilities|Array|Add (Variables|Default|GetFreeObjects) Object))

(fn ConstructionScript)