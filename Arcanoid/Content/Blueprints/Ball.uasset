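; Ball actor that travels in a random 2D direction and bounces off whatever it hits, as in a Pong-style game.
; On BeginPlay it picks a normalized start direction with limited vertical spread.
; Each Tick it moves by a swept world offset of Direction times Speed, with no delta time scaling, and on a blocking hit reflects Direction off the surface normal.
; GetSpeedDifference holds only an unused multiply.
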(event EventTick
  (params (DeltaSeconds :type Float%20%28single-precision%29))
  (bind _sweephitresult (Transformation|AddActorWorldOffset (* (Variables|Default|GetDirection) (Variables|Default|GetSpeed)) true))
  (if (.bblockinghit _sweephitresult)
    (Variables|Default|SetDirection (Class|KismetMathLibrary|VectorNormal2D (Math|Vector|GetReflectionVector (Variables|Default|GetDirection) (.normal _sweephitresult)) 0.0001))))

(event EventBeginPlay
  (Variables|Default|SetDirection (Class|KismetMathLibrary|VectorNormal2D (Math|Vector|MakeVector (Math|Random|RandomFloat) (Math|Random|RandomFloatinRange -0.5 0.5) 0.0) 0.0001)))

(fn ConstructionScript)